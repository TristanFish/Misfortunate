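; Parent Blueprint for road intersections in a procedural road generator, providing connector points where roads attach.
; The construction script builds labeled arrow connectors, caches their world transforms and optionally applies seeded random materials by slot name.
; Utility functions use those transforms to spawn or move roads, or snap spline ends with length-scaled tangents.
; Experimental bulk spawning sphere-traces each connector for existing roads, and a landscape tool flattens terrain along a spline.
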(fn ConstructionScript
  (Utilities|FlowControl|Sequence
    (:then_0
      (CallFunction|AddConnectors))
    (:then_1
      (if (Variables|Material|GetRandomize%20Material)
        (Class|KismetMathLibrary|SeedRandomStream (Variables|Material|GetMaterial%20Seed)))
      (Variables|Material|SetRandomize%20Material false))
    (:then_2
      (if (Variables|Material|GetCan%20Override%20Material)
        (CallFunction|SetMeshMaterial (Variables|Material|GetMaterial%20Manager) (Variables|Default|GetIntersection_Mesh%20Ref) (Variables|Material|GetMaterial%20Seed))))))

(fn ConnectRoadStartatChoosenConnector
  (Utilities|IsValid (Variables|RoadConnectionSystem|GetRoad%20To%20Connect)
    (:Is%20Valid
      (LocalVariables|SetRoad%20Spline (Variables|/Game/ProceduralRoadGenerator/ProceduralRoadGenerator_BP.ProceduralRoadGenerator_BP_C|GetSpline (Variables|RoadConnectionSystem|GetRoad%20To%20Connect)))
      (LocalVariables|SetPoint%20To%20Connect (Class|KismetSystemLibrary|MakeLiteralInteger))
      (Spline|SetLocationatSplinePoint (LocalVariables|GetRoad%20Spline) (LocalVariables|GetPoint%20To%20Connect) (.location (Utilities|Array|Get(acopy) (Variables|Default|GetConnectors%20Location%20Array) (Variables|Default|GetConnectors%20ID%20To%20Connect))) "World" true)
      (Spline|SetTangentatSplinePoint (LocalVariables|GetRoad%20Spline) (LocalVariables|GetPoint%20To%20Connect) (* (Math|Vector|GetForwardVector (.rotation (Utilities|Array|Get(acopy) (Variables|Default|GetConnectors%20Location%20Array) (Variables|Default|GetConnectors%20ID%20To%20Connect)))) (/ (Spline|GetSplineLength (LocalVariables|GetRoad%20Spline)) (Math|Conversions|ToFloat(Integer) (select (== (Math|Float|Round (/ (Spline|GetSplineLength (LocalVariables|GetRoad%20Spline)) (Variables|/Game/ProceduralRoadGenerator/ProceduralRoadGenerator_BP.ProceduralRoadGenerator_BP_C|GetRoad%20World%20Length (Variables|RoadConnectionSystem|GetRoad%20To%20Connect)))) 0) 1 (Math|Float|Round (/ (Spline|GetSplineLength (LocalVariables|GetRoad%20Spline)) (Variables|/Game/ProceduralRoadGenerator/ProceduralRoadGenerator_BP.ProceduralRoadGenerator_BP_C|GetRoad%20World%20Length (Variables|RoadConnectionSystem|GetRoad%20To%20Connect)))))))) "World" true)
      (Development|PrintString (Utilities|String|Append (Utilities|GetObjectName (Variables|RoadConnectionSystem|GetRoad%20To%20Connect)) " succesfully connected to connector " (Utilities|String|ToString(Integer) (Variables|Default|GetConnectors%20ID%20To%20Connect))) true true "(R=0.000000,G=1.000000,B=0.000000,A=1.000000)" (Variables|RoadConnectionSystem|GetOn%20Screen%20Text%20Display%20Delay)))
    (:Is%20Not%20Valid
      (Development|PrintString "Specify road to connect" true true "(R=1.000000,G=0.000000,B=0.000000,A=1.000000)" (Variables|RoadConnectionSystem|GetOn%20Screen%20Text%20Display%20Delay)))))

(fn MoveRoadatChoosenConnector
  (Utilities|IsValid (Variables|RoadConnectionSystem|GetRoad%20To%20Connect)
    (:Is%20Valid
      (bind _returnvalue (Transformation|SetActorTransform (Variables|RoadConnectionSystem|GetRoad%20To%20Connect) (Utilities|Array|Get(acopy) (Variables|Default|GetConnectors%20Location%20Array) (Variables|Default|GetConnectors%20ID%20To%20Connect))))
      (if _returnvalue
        (Development|PrintString (Utilities|String|Append (Utilities|GetObjectName (Variables|RoadConnectionSystem|GetRoad%20To%20Connect)) " succesfully moved to connector " (Utilities|String|ToString(Integer) (Variables|Default|GetConnectors%20ID%20To%20Connect))) true true "(R=0.000000,G=1.000000,B=0.000000,A=1.000000)" (Variables|RoadConnectionSystem|GetOn%20Screen%20Text%20Display%20Delay))))
    (:Is%20Not%20Valid
      (Development|PrintString "Specify road to move" true true "(R=1.000000,G=0.000000,B=0.000000,A=1.000000)" (Variables|RoadConnectionSystem|GetOn%20Screen%20Text%20Display%20Delay)))))

(fn SpawnRoadatChoosenConnector
  (Game|SpawnActorfromClass (Variables|RoadConnectionSystem|GetRoad%20To%20Spawn) (Utilities|Array|Get(acopy) (Variables|Default|GetConnectors%20Location%20Array) (Variables|Default|GetConnectors%20ID%20To%20Connect)) "Undefined" 0 0)
  (Development|PrintString (Utilities|String|Append "Succesfully spawned road at connector " (Utilities|String|ToString(Integer) (Variables|Default|GetConnectors%20ID%20To%20Connect))) true true "(R=0.000000,G=1.000000,B=0.000000,A=1.000000)" (Variables|RoadConnectionSystem|GetOn%20Screen%20Text%20Display%20Delay)))

(fn SetConnectorsTransform
  (params (Total%20Number%20Of%20Connectors :type Integer))
  (for _index (range 0 (- Total%20Number%20Of%20Connectors 1))
    (LocalVariables|SetCurrent%20Loop%20Index _index)
    (Utilities|Array|SetArrayElem (Variables|Default|GetConnectors%20Location%20Array) (LocalVariables|GetCurrent%20Loop%20Index) (Transformation|GetWorldTransform (Utilities|Select :Index (LocalVariables|GetCurrent%20Loop%20Index) :Option%200 0 :Option%201 0 :Option%202 0 :Option%203 0 :Option%204 0 :Option%205 0)) true))
  (Utilities|Array|Resize (Variables|Default|GetConnectors%20Location%20Array) Total%20Number%20Of%20Connectors))

(fn SpawnRoadsatAllConnectors
  (for (_array_element _array_index) (Variables|Default|GetConnectors%20Location%20Array)
    ;[1 1 1] Experimental
    (bind (_outhits _returnvalue) (Collision|MultiSphereTraceForObjects (.Location (Math|Transform|BreakTransform _array_element)) (+ (.Location (Math|Transform|BreakTransform _array_element)) 5.0) (Variables|Default|GetTrace%20Radius) (Utilities|Array|MakeArray "ObjectTypeQuery1") false 0 "ForDuration" true "(R=1.000000,G=0.000000,B=0.000000,A=1.000000)" "(R=0.000000,G=1.000000,B=0.000000,A=1.000000)" (Variables|RoadConnectionSystem|GetOn%20Screen%20Text%20Display%20Delay)))
    (if _returnvalue
      (bind (_array_element_2 _array_index_2) (Utilities|Array|ForEachLoopwithBreak _outhits :!label _label)
        (:LoopBody
          (if (== (.hitactor _array_element_2) "/Game/ProceduralRoadGenerator/ProceduralRoadGenerator_BP.ProceduralRoadGenerator_BP")
            (goto _label Break)
            (elif (== _array_index_2 (- (Utilities|Array|Length _outhits) 1))
              (Game|SpawnActorfromClass (Variables|RoadConnectionSystem|GetRoad%20To%20Spawn) (Math|Transform|MakeTransform (.Location (Math|Transform|BreakTransform _array_element)) (.Rotation (Math|Transform|BreakTransform _array_element)) (.Scale (Math|Transform|BreakTransform _array_element))) "AlwaysSpawn" 0 0 :!label _label_2)
              (Development|PrintString (Utilities|String|Append "Road Spawned Succesfully at con: " (Utilities|String|ToString(Integer) _array_index)) true true "(R=0.000000,G=1.000000,B=0.000000,A=1.000000)" (Variables|RoadConnectionSystem|GetOn%20Screen%20Text%20Display%20Delay))))))
      (else
        (goto _label_2)))))

(fn FlattenLandscape
  (bind _landscapeto_deform (Variables|Landscape|GetLandscapeTo%20Deform))
  (bind _road_side_falloff (Variables|Landscape|GetRoad%20Side%20Falloff))
  (bind _road_width (Variables|Landscape|GetRoad%20Width))
  (Utilities|IsValid (Variables|Landscape|GetLandscapeTo%20Deform)
    (:Is%20Valid
      (if (Variables|Landscape|GetPrevent%20High%20values)
        (if (not (Math|Boolean|ORBoolean (>= (Variables|Landscape|GetNum%20Of%20Divisions) 3000) (>= (Variables|Landscape|GetRoad%20Width) 3e+03) (>= (Variables|Landscape|GetRoad%20Side%20Falloff) 3e+03)))
          (Landscape|Editor|EditorApplySpline _landscapeto_deform (Variables|Default|GetSpline) _road_width _road_width _road_side_falloff _road_side_falloff 0.0 0.0 (Variables|Landscape|GetNum%20Of%20Divisions) (Variables|Landscape|GetCan%20Raise%20Landscape) (Variables|Landscape|GetCan%20Lower%20Landscape) 0 :!label _label)
          (Development|PrintString (Utilities|String|Append (Utilities|GetObjectName _landscapeto_deform) " has been adjusted succesfully by " (Utilities|GetObjectName self)) true true "(R=0.000000,G=1.000000,B=0.000000,A=1.000000)" 3.0))
        (else
          (goto _label))))
    (:Is%20Not%20Valid
      (Development|PrintString "Specify landscape to deform" true true "(R=1.000000,G=0.000000,B=0.000000,A=1.000000)" 3.0))))

(fn SetMeshMaterial
  (params (Material :type Array%20of%20Material%20Attribute%20Structures) (Target%20Mesh :type Static%20Mesh%20Component%20Object%20Reference) (Seed :type Random%20Stream%20Structure))
  (bind _returnvalue (Utilities|Array|Length Material))
  (LocalVariables|SetTarget%20Mesh%20 Target%20Mesh)
  (if (> _returnvalue 0)
    (for _index (range 0 (Math|Integer|Min(Integer) (- _returnvalue 1) (Rendering|Material|GetNumMaterials (LocalVariables|GetTarget%20Mesh%20))))
      (if (> (Utilities|Array|Length (.materialslotname (Utilities|Array|Get(acopy) Material _index))) 0)
        (for _index_2 (range 0 (- (Utilities|Array|Length (.materialslotname (Utilities|Array|Get(acopy) Material _index))) 1))
          (Rendering|Material|SetMaterialbyName (LocalVariables|GetTarget%20Mesh%20) (Utilities|Array|Get(acopy) (.materialslotname (Utilities|Array|Get(acopy) Material _index)) _index_2) (Utilities|Array|Get(acopy) (.material (Utilities|Array|Get(acopy) Material _index)) (Math|Random|RandomIntegerinRangefromStream 0 (- (Utilities|Array|Length (.material (Utilities|Array|Get(acopy) Material _index))) 1) (Math|Random|MakeRandomStream (.initialseed Seed))))))))))

(fn AddConnectors
  (bind _connectors_manager (Variables|ConnectorsSetting|GetConnectors%20Manager))
  (bind _returnvalue (Utilities|Array|Length _connectors_manager))
  (Utilities|Array|Resize (Variables|Default|GetConnectors%20Location%20Array) _returnvalue)
  (for _index (range 0 (- _returnvalue 1))
    (LocalVariables|SetIndex _index)
    (bind _returnvalue_2 (AddComponent|AddTextRenderComponent false (Math|Transform|MakeTransform (.connectorlocation (Utilities|Array|Get(acopy) (Variables|ConnectorsSetting|GetConnectors%20Manager) (LocalVariables|GetIndex))) (.connectorrotation (Utilities|Array|Get(acopy) (Variables|ConnectorsSetting|GetConnectors%20Manager) (LocalVariables|GetIndex))) (.connectorscale (Utilities|Array|Get(acopy) (Variables|ConnectorsSetting|GetConnectors%20Manager) (LocalVariables|GetIndex))))))
    (LocalVariables|SetText%20Render%20Ref _returnvalue_2)
    (Rendering|Components|TextRender|SetText (LocalVariables|GetText%20Render%20Ref) (.connectorname (Utilities|Array|Get(acopy) (Variables|ConnectorsSetting|GetConnectors%20Manager) (LocalVariables|GetIndex))))
    (Rendering|Components|TextRender|SetWorldSize (LocalVariables|GetText%20Render%20Ref) (Variables|RoadConnectionSystem|GetText%20Size))
    (Rendering|SetVisibility (LocalVariables|GetText%20Render%20Ref) (Variables|RoadConnectionSystem|GetSet%20Connectors%20Text%20Visibilty) false)
    (bind _returnvalue_3 (AddComponent|AddArrowComponent false (Math|Transform|MakeTransform (.connectorlocation (Utilities|Array|Get(acopy) (Variables|ConnectorsSetting|GetConnectors%20Manager) (LocalVariables|GetIndex))) (.connectorrotation (Utilities|Array|Get(acopy) (Variables|ConnectorsSetting|GetConnectors%20Manager) (LocalVariables|GetIndex))) (.connectorscale (Utilities|Array|Get(acopy) (Variables|ConnectorsSetting|GetConnectors%20Manager) (LocalVariables|GetIndex))))))
    (Rendering|SetVisibility _returnvalue_3 (Variables|RoadConnectionSystem|GetSet%20Connectors%20Text%20Visibilty) false)
    (Components|Arrow|SetArrowColor(LinearColor) _returnvalue_3 (.color (Utilities|Array|Get(acopy) (Variables|ConnectorsSetting|GetConnectors%20Manager) (LocalVariables|GetIndex))))
    (Rendering|Components|TextRender|SetTextRenderColor (LocalVariables|GetText%20Render%20Ref) (Math|Conversions|ToColor(LinearColor) (.color (Utilities|Array|Get(acopy) (Variables|ConnectorsSetting|GetConnectors%20Manager) (LocalVariables|GetIndex)))))
    (Utilities|Array|SetArrayElem (Variables|Default|GetConnectors%20Location%20Array) (LocalVariables|GetIndex) (Math|Transform|MakeTransform (.location (Math|Transform|ComposeTransforms (Math|Transform|MakeTransform (.connectorlocation (Utilities|Array|Get(acopy) (Variables|ConnectorsSetting|GetConnectors%20Manager) (LocalVariables|GetIndex))) (.connectorrotation (Utilities|Array|Get(acopy) (Variables|ConnectorsSetting|GetConnectors%20Manager) (LocalVariables|GetIndex))) (.connectorscale (Utilities|Array|Get(acopy) (Variables|ConnectorsSetting|GetConnectors%20Manager) (LocalVariables|GetIndex)))) (Transformation|GetActorTransform))) (.rotation (Math|Transform|ComposeTransforms (Math|Transform|MakeTransform (.connectorlocation (Utilities|Array|Get(acopy) (Variables|ConnectorsSetting|GetConnectors%20Manager) (LocalVariables|GetIndex))) (.connectorrotation (Utilities|Array|Get(acopy) (Variables|ConnectorsSetting|GetConnectors%20Manager) (LocalVariables|GetIndex))) (.connectorscale (Utilities|Array|Get(acopy) (Variables|ConnectorsSetting|GetConnectors%20Manager) (LocalVariables|GetIndex)))) (Transformation|GetActorTransform))) (Transformation|GetActorScale3D)))))

(fn ConnectRoadEndatChoosenConnector
  (Utilities|IsValid (Variables|RoadConnectionSystem|GetRoad%20To%20Connect)
    (:Is%20Valid
      (LocalVariables|SetRoad%20Spline (Variables|/Game/ProceduralRoadGenerator/ProceduralRoadGenerator_BP.ProceduralRoadGenerator_BP_C|GetSpline (Variables|RoadConnectionSystem|GetRoad%20To%20Connect)))
      (LocalVariables|SetPoint%20To%20Connect (- (Spline|GetNumberOfSplinePoints (LocalVariables|GetRoad%20Spline)) 1))
      (Spline|SetLocationatSplinePoint (LocalVariables|GetRoad%20Spline) (LocalVariables|GetPoint%20To%20Connect) (.location (Utilities|Array|Get(acopy) (Variables|Default|GetConnectors%20Location%20Array) (Variables|Default|GetConnectors%20ID%20To%20Connect))) "World" true)
      (Spline|SetTangentatSplinePoint (LocalVariables|GetRoad%20Spline) (LocalVariables|GetPoint%20To%20Connect) (* (Math|Vector|GetForwardVector (Math|Rotator|CombineRotators (.rotation (Utilities|Array|Get(acopy) (Variables|Default|GetConnectors%20Location%20Array) (Variables|Default|GetConnectors%20ID%20To%20Connect))) "0,180.000000, 0")) (/ (Spline|GetSplineLength (LocalVariables|GetRoad%20Spline)) (Math|Conversions|ToFloat(Integer) (select (== (Math|Float|Round (/ (Spline|GetSplineLength (LocalVariables|GetRoad%20Spline)) (Variables|/Game/ProceduralRoadGenerator/ProceduralRoadGenerator_BP.ProceduralRoadGenerator_BP_C|GetRoad%20World%20Length (Variables|RoadConnectionSystem|GetRoad%20To%20Connect)))) 0) 1 (Math|Float|Round (/ (Spline|GetSplineLength (LocalVariables|GetRoad%20Spline)) (Variables|/Game/ProceduralRoadGenerator/ProceduralRoadGenerator_BP.ProceduralRoadGenerator_BP_C|GetRoad%20World%20Length (Variables|RoadConnectionSystem|GetRoad%20To%20Connect)))))))) "World" true)
      (Development|PrintString (Utilities|String|Append (Utilities|GetObjectName (Variables|RoadConnectionSystem|GetRoad%20To%20Connect)) " succesfully connected to connector " (Utilities|String|ToString(Integer) (Variables|Default|GetConnectors%20ID%20To%20Connect))) true true "(R=0.000000,G=1.000000,B=0.000000,A=1.000000)" (Variables|RoadConnectionSystem|GetOn%20Screen%20Text%20Display%20Delay)))
    (:Is%20Not%20Valid
      (Development|PrintString "Specify road to connect" true true "(R=1.000000,G=0.000000,B=0.000000,A=1.000000)" (Variables|RoadConnectionSystem|GetOn%20Screen%20Text%20Display%20Delay)))))