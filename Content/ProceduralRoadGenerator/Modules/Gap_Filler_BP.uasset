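; Procedural road generator actor that fills gaps by turning a spline outline into a triangulated procedural mesh.
; Its construction script builds vertices from spline points, bounds-normalized UVs, tangents, optional collision and a seeded random material, with optional point-number labels.
; A Z-flip works around a collision issue.
; A separate CopyRoadSplinePoints function rebuilds the outline from referenced roads as linear points, using neighbor direction dot products to handle point order.
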(event EventBeginPlay)

(event Collision|EventActorBeginOverlap
  (params (OtherActor :type Actor%20Object%20Reference)))

(event EventTick
  (params (DeltaSeconds :type Float%20%28single-precision%29)))

(fn ConstructionScript
  (Utilities|FlowControl|Sequence
    (:then_0
      (if (Variables|Setup|GetRandomize%20Material)
        (Class|KismetMathLibrary|SeedRandomStream (Variables|Setup|GetMaterial%20%20Seed)))
      (Variables|Setup|SetRandomize%20Material false))
    (:then_1
      (Spline|SetClosedLoop (Variables|Default|GetSpline) (Variables|Setup|GetClose%20Spline) true)
      ;[1 1 1] Get Actor Bound Used to normalize UV, we first reset actor rotation so it don't affects the bound
      (Variables|Default|SetRotation%20Backup (Transformation|GetActorRotation))
      (Transformation|SetActorRotation "0, 0, 0")
      (Variables|Default|SetBound (.BoxExtent (Collision|GetComponentBounds (Variables|Default|GetSpline))))
      (Transformation|SetActorRotation (Variables|Default|GetRotation%20Backup))
      ;[1 1 1] Add Procedural Mesh
      (CallFunction|AddProceduralMesh 0.0)
      ;[1 1 1] Spline Point Text
      (if (Variables|Setup|GetShow%20Spline%20Point%20Number)
        (for _index (range 0 (- (Spline|GetNumberOfSplinePoints (Variables|Default|GetSpline)) 1))
          (bind _returnvalue (AddComponent|AddTextRenderComponent false (Spline|GetTransformatSplinePoint (Variables|Default|GetSpline) _index "Local" false)))
          (Rendering|Components|TextRender|SetText _returnvalue (Utilities|Text|ToText(Integer) _index))
          (Rendering|Components|TextRender|SetWorldSize _returnvalue 2e+03))))))

(fn AddProceduralMesh
  (params (Height%20Offset :type Float%20%28single-precision%29))
  (bind _bound (Variables|Default|GetBound))
  (bind _bound_2 (Variables|Default|GetBound))
  (LocalVariables|SetMaterial%20Array%20Lenght (Utilities|Array|Length (Variables|Setup|GetMaterial)))
  (Variables|Default|SetNumber%20Of%20Spline%20Point (Spline|GetNumberOfSplinePoints (Variables|Default|GetSpline)))
  (Transformation|SetRelativeTransform (Variables|Default|GetProceduralMesh) (select (Variables|Setup|GetFix%20Collision%20Issue) (Math|Transform|MakeTransform "0, 0, 0" "0, 0, 0" "1,1,-1.000000") "") false false)
  (Utilities|Array|Resize (Variables|Default|GetVertex) (Variables|Default|GetNumber%20Of%20Spline%20Point))
  (Utilities|Array|Resize (Variables|Default|GetUV%200) (Variables|Default|GetNumber%20Of%20Spline%20Point))
  (Utilities|Array|Resize (Variables|Default|GetUV%201) (Variables|Default|GetNumber%20Of%20Spline%20Point))
  (Rendering|SetCastShadow (Variables|Default|GetProceduralMesh) (Variables|Setup|GetCan%20Cast%20Shadow))
  (Transformation|AddLocalOffset (Variables|Default|GetProceduralMesh) (Math|Vector|MakeVector 0.0 0.0 Height%20Offset) false false)
  (for _index (range 0 (- (Variables|Default|GetNumber%20Of%20Spline%20Point) 1))
    (Variables|Default|SetCurrent%20Spline%20Point%20Index _index)
    ;[1 1 1] Vertex
    (Utilities|Array|SetArrayElem (Variables|Default|GetVertex) (Variables|Default|GetCurrent%20Spline%20Point%20Index) (Math|Vector|MakeVector (.x (Spline|GetLocationatSplinePoint (Variables|Default|GetSpline) (Variables|Default|GetCurrent%20Spline%20Point%20Index) "Local")) (.y (Spline|GetLocationatSplinePoint (Variables|Default|GetSpline) (Variables|Default|GetCurrent%20Spline%20Point%20Index) "Local")) (* (select (Variables|Setup|GetFix%20Collision%20Issue) -1 1) (.z (Spline|GetLocationatSplinePoint (Variables|Default|GetSpline) (Variables|Default|GetCurrent%20Spline%20Point%20Index) "Local")))))
    ;[1 1 1] UV 0
    (Utilities|Array|SetArrayElem (Variables|Default|GetUV%200) (Variables|Default|GetCurrent%20Spline%20Point%20Index) (* (Math|Vector2D|MakeVector2D (/ (.x (Utilities|Array|Get(acopy) (Variables|Default|GetVertex) (Variables|Default|GetCurrent%20Spline%20Point%20Index))) (Math|Float|Max(Float) (.x _bound_2) 0.1)) (/ (.y (Utilities|Array|Get(acopy) (Variables|Default|GetVertex) (Variables|Default|GetCurrent%20Spline%20Point%20Index))) (Math|Float|Max(Float) (.y _bound_2) 0.1))) (Variables|Setup|GetUV%20Multiplier)))
    ;[1 1 1] UV 1
    (Utilities|Array|SetArrayElem (Variables|Default|GetUV%201) (Variables|Default|GetCurrent%20Spline%20Point%20Index) (Math|Vector2D|MakeVector2D (/ (.x (Utilities|Array|Get(acopy) (Variables|Default|GetVertex) (Variables|Default|GetCurrent%20Spline%20Point%20Index))) (Math|Float|Max(Float) (.x _bound) 0.1)) (/ (.y (Utilities|Array|Get(acopy) (Variables|Default|GetVertex) (Variables|Default|GetCurrent%20Spline%20Point%20Index))) (Math|Float|Max(Float) (.y _bound) 0.1)))))
  ;[1 1 1] Create Triangle
  (bind _triangles (CallFunction|TriangulatePolygon (Variables|Default|GetVertex)))
  (Variables|Default|SetTriangle _triangles)
  (Utilities|FlowControl|Sequence
    (:then_0
      ;[1 1 1] Remove invalid triangle created by   "triangulate function"
      (Utilities|Array|Resize (Variables|Default|GetTriangle) (- (Utilities|Array|Length (Variables|Default|GetTriangle)) 3)))
    (:then_1
      ;[1 1 1] Calculate Tangents and Normals
      (bind (_normals _tangents) (Class|KismetProceduralMeshLibrary|CalculateTangentsforMesh (Variables|Default|GetVertex) (Variables|Default|GetTriangle) (Variables|Default|GetUV%200)))
      ;[1 1 1] Create Mesh
      (Class|ProceduralMeshComponent|CreateMeshSectionLinearColor (Variables|Default|GetProceduralMesh) 0 (Variables|Default|GetVertex) (Variables|Default|GetTriangle) _normals (Variables|Default|GetUV%200) (Variables|Default|GetUV%201) 0 0 0 _tangents (Variables|Setup|GetAdd%20Collision))
      ;[1 1 1] Assign Material
      (if (> (LocalVariables|GetMaterial%20Array%20Lenght) 0)
        (Rendering|Material|SetMaterial (Variables|Default|GetProceduralMesh) 0 (Utilities|Array|Get(acopy) (Variables|Setup|GetMaterial) (Math|Random|RandomIntegerinRangefromStream 0 (- (LocalVariables|GetMaterial%20Array%20Lenght) 1) (Math|Random|MakeRandomStream (.initialseed (Variables|Setup|GetMaterial%20%20Seed))))))))))

(fn CopyRoadSplinePoints
  (bind _forward_vector (Variables|Default|GetForward%20Vector))
  (bind _returnvalue (Utilities|Array|Length _forward_vector))
  (Utilities|Array|Clear (Variables|Default|GetSpline%20Points))
  (Utilities|Array|Clear (Variables|Default|GetForward%20Vector))
  (Utilities|Array|Clear (Variables|Default|GetRight%20Vector))
  (Utilities|Array|Clear (Variables|Default|GetDot%20))
  (for _index (range 0 (- (Utilities|Array|Length (Variables|Default|GetRoad%20Spline%20To%20Copy)) 1))
    (LocalVariables|SetCurrent%20Road%20Index _index)
    (bind _output_get (LocalVariables|SetCurrent%20Road (Utilities|Array|Get(acopy) (Variables|Default|GetRoad%20Spline%20To%20Copy) (LocalVariables|GetCurrent%20Road%20Index))))
    (Utilities|IsValid _output_get
      (:Is%20Valid
        (Utilities|Array|SetArrayElem (Variables|Default|GetForward%20Vector) (LocalVariables|GetCurrent%20Road%20Index) (Math|Vector|GetForwardVector (Variables|/Game/ProceduralRoadGenerator/ProceduralRoadGenerator_BP.ProceduralRoadGenerator_BP_C|GetSpline (LocalVariables|GetCurrent%20Road))) true)
        (Utilities|Array|SetArrayElem (Variables|Default|GetRight%20Vector) (LocalVariables|GetCurrent%20Road%20Index) (Math|Vector|GetRightVector (Variables|/Game/ProceduralRoadGenerator/ProceduralRoadGenerator_BP.ProceduralRoadGenerator_BP_C|GetSpline (LocalVariables|GetCurrent%20Road))) true))
      (:Is%20Not%20Valid
        (Development|PrintString (Utilities|String|Append "road in " (Utilities|String|ToString(Integer) (LocalVariables|GetCurrent%20Road%20Index)) " is invalid, please make sure to set a road")))))
  (Utilities|Array|Resize _forward_vector (+ _returnvalue 1))
  (Utilities|Array|Resize (Variables|Default|GetRight%20Vector) _returnvalue)
  (for _index_2 (range 0 (- _returnvalue 2))
    (Utilities|Array|SetArrayElem (Variables|Default|GetDot%20) (+ _index_2 1) (Math|Vector2D|DotProduct(2D) (Math|Vector2D|MakeVector2D (.x (Utilities|Array|Get(acopy) (Variables|Default|GetForward%20Vector) _index_2)) (.y (Utilities|Array|Get(acopy) (Variables|Default|GetForward%20Vector) _index_2))) (Math|Vector2D|MakeVector2D (.x (Utilities|Array|Get(acopy) (Variables|Default|GetRight%20Vector) (+ _index_2 1))) (.y (Utilities|Array|Get(acopy) (Variables|Default|GetRight%20Vector) (+ _index_2 1))))) true))
  (for _index_3 (range 0 (- (Utilities|Array|Length (Variables|Default|GetRoad%20Spline%20To%20Copy)) 1))
    (LocalVariables|SetCurrent%20Road%20Index _index_3)
    (bind _output_get_2 (LocalVariables|SetCurrent%20Road (Utilities|Array|Get(acopy) (Variables|Default|GetRoad%20Spline%20To%20Copy) (LocalVariables|GetCurrent%20Road%20Index))))
    (Utilities|IsValid _output_get_2
      (:Is%20Valid
        (for _index_4 (range 0 (- (Spline|GetNumberOfSplinePoints (Variables|/Game/ProceduralRoadGenerator/ProceduralRoadGenerator_BP.ProceduralRoadGenerator_BP_C|GetSpline (LocalVariables|GetCurrent%20Road))) 1))
          (LocalVariables|SetCurrent%20Road%20Spline%20Point%20Index _index_4)
          (Utilities|Array|SetArrayElem (Variables|Default|GetSpline%20Points) (+ (LocalVariables|GetTotal%20Road%20Spline%20Points) (LocalVariables|GetCurrent%20Road%20Spline%20Point%20Index)) (Spline|GetLocationatSplinePoint (Variables|/Game/ProceduralRoadGenerator/ProceduralRoadGenerator_BP.ProceduralRoadGenerator_BP_C|GetSpline (LocalVariables|GetCurrent%20Road)) (LocalVariables|GetCurrent%20Road%20Spline%20Point%20Index) "World") true)
          (Utilities|Array|SetArrayElem (Variables|Default|GetCurrent%20Road%20Spline%20Point) (LocalVariables|GetCurrent%20Road%20Spline%20Point%20Index) (Spline|GetLocationatSplinePoint (Variables|/Game/ProceduralRoadGenerator/ProceduralRoadGenerator_BP.ProceduralRoadGenerator_BP_C|GetSpline (LocalVariables|GetCurrent%20Road)) (LocalVariables|GetCurrent%20Road%20Spline%20Point%20Index) "World") true))
        (Utilities|FlowControl|Sequence
          (:then_0
            (if (> (Utilities|Array|Get(acopy) (Variables|Default|GetDot%20) (LocalVariables|GetCurrent%20Road%20Index)) 0.0)
              (bind (_arrayindex _arrayelement) (Utilities|Array|ReverseforEachLoop (Variables|Default|GetCurrent%20Road%20Spline%20Point))
                (:LoopBody
                  (LocalVariables|SetCurrent%20Road%20Spline%20Point%20Index _arrayindex)
                  (Utilities|Array|SetArrayElem (Variables|Default|GetSpline%20Points) (+ (LocalVariables|GetTotal%20Road%20Spline%20Points) (LocalVariables|GetCurrent%20Road%20Spline%20Point%20Index) 1) _arrayelement true))
                (:Completed
                  (Development|PrintString "executed")))))
          (:then_1
            (LocalVariables|SetTotal%20Road%20Spline%20Points (+ (LocalVariables|GetCurrent%20Road%20Spline%20Point%20Index) (LocalVariables|GetTotal%20Road%20Spline%20Points) 1)))))))
  (LocalVariables|SetTotal%20Road%20Spline%20Points 0)
  (Spline|ClearSplinePoints (Variables|Default|GetSpline) true)
  (Spline|SetSplinePoints (Variables|Default|GetSpline) (Variables|Default|GetSpline%20Points) "World" true)
  (for _index_5 (range 0 (- (Utilities|Array|Length (Variables|Default|GetSpline%20Points)) 1))
    (Spline|SetSplinePointType (Variables|Default|GetSpline) _index_5 "Linear" true)))