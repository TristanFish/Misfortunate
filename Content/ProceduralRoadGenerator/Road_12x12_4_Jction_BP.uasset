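; Four-way 12x12 road junction piece for the procedural road generator, built as a child Blueprint.
; Its construction script stores the selected connectors option as an integer ID and assigns the four-way intersection static mesh.
; It then calls the parent construction script, so those values are set before any inherited logic runs.
; The event graph holds only disabled default events.
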(event EventBeginPlay
  (|CallParentFunction) ; This node is disabled and will not be called.\nDrag off pins to build functionality.
)

(event Collision|EventActorBeginOverlap
  (params (OtherActor :type Actor%20Object%20Reference))
  (|CallParentFunction OtherActor) ; This node is disabled and will not be called.\nDrag off pins to build functionality.
)

(event EventTick
  (params (DeltaSeconds :type Float%20%28single-precision%29))
  (|CallParentFunction DeltaSeconds) ; This node is disabled and will not be called.\nDrag off pins to build functionality.
)

(fn ConstructionScript
  (Variables|Default|SetConnectors%20ID%20To%20Connect (Math|Conversions|ToInteger(Byte) (Variables|RoadConnectionSystem|GetSelect%20Connectors)))
  (Components|StaticMesh|SetStaticMesh (Variables|Default|GetIntersection_Mesh%20Ref) "/Game/ProceduralRoadGenerator/Meshes/Road/Road_12x12_4_Way_Intersection_Set.Road_12x12_4_Way_Intersection_Set")
  (|CallParentFunction))