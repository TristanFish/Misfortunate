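; Telephone box prop whose door swings open when something overlaps its trigger box and closes when the overlap ends.
; A timeline drives the door's yaw, scaled by a speed multiplier and clamped.
; The construction script tints the rect light and a dynamic light-box glass material with one color from three seeded streams.
; A self-resetting RandomizeLightColor toggle re-seeds those streams, so the color otherwise stays stable across reconstruction.
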(event OnComponentBeginOverlap(Box)
  (params (OverlappedComponent :type Primitive%20Component%20Object%20Reference) (OtherActor :type Actor%20Object%20Reference) (OtherComp :type Primitive%20Component%20Object%20Reference) (OtherBodyIndex :type Integer) (bFromSweep :type Boolean) (SweepResult :type Hit%20Result%20Structure%20%28by%20ref%29))
  (bind _door_angle (Timeline|Timeline_0 Play)
    (:Update
      (CallFunction|OpenDoor (Variables|Default|GetTelephone_Box_Door) (* _door_angle (Variables|Default|GetDoor%20Opening%20Speed))))))

(event OnComponentEndOverlap(Box)
  (params (OverlappedComponent :type Primitive%20Component%20Object%20Reference) (OtherActor :type Actor%20Object%20Reference) (OtherComp :type Primitive%20Component%20Object%20Reference) (OtherBodyIndex :type Integer))
  (bind _door_angle (Timeline|Timeline_0 Reverse)
    (:Update
      (CallFunction|OpenDoor (Variables|Default|GetTelephone_Box_Door) (* _door_angle (Variables|Default|GetDoor%20Opening%20Speed))))))

(fn ConstructionScript
  (Utilities|FlowControl|Sequence
    (:then_0
      (if (Variables|Default|GetRandomize%20Light%20Color)
        (Class|KismetMathLibrary|SeedRandomStream (Variables|Default|GetRed%20Seed))
        (Class|KismetMathLibrary|SeedRandomStream (Variables|Default|GetGreen%20Seed))
        (Class|KismetMathLibrary|SeedRandomStream (Variables|Default|GetBlue%20Seed))
        (Variables|Default|SetRandomize%20Light%20Color false)))
    (:then_1
      (LocalVariables|SetColor (Math|Color|MakeColor (Math|Random|RandomFloatinRangefromStream 0.2 1.0 (Math|Random|MakeRandomStream (.initialseed (Variables|Default|GetRed%20Seed)))) (Math|Random|RandomFloatinRangefromStream 0.2 1.0 (Math|Random|MakeRandomStream (.initialseed (Variables|Default|GetGreen%20Seed)))) (Math|Random|RandomFloatinRangefromStream 0.2 1.0 (Math|Random|MakeRandomStream (.initialseed (Variables|Default|GetBlue%20Seed))))))
      (Rendering|Components|Light|SetLightColor (Variables|Default|GetRectLight) (LocalVariables|GetColor) true)
      (bind _returnvalue (Rendering|Material|CreateDynamicMaterialInstance (Variables|Default|GetLight_Box) 0 "/Game/ProceduralRoadGenerator/Material/Glass/Opaque_Glass_inst5.Opaque_Glass_inst5" "None" :!class /Script/Engine.PrimitiveComponent))
      (Rendering|Material|SetVectorParameterValue _returnvalue "Uniform Color" (LocalVariables|GetColor) :!class /Script/Engine.MaterialInstanceDynamic))))

(fn OpenDoor
  (params (Door%20Mesh :type Scene%20Component%20Object%20Reference) (Value :type Float%20%28double-precision%29))
  (bind _relativerotation (Variables|/Script/Engine.SceneComponent|GetRelativeRotation Door%20Mesh))
  (Transformation|SetRelativeRotation Door%20Mesh (Math|Rotator|MakeRotator (.roll _relativerotation) (.pitch _relativerotation) (Math|Float|Clamp(Float) Value -9e+01 9e+01)) false false))