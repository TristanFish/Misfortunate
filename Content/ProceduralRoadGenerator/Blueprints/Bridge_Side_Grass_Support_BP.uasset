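; Bridge side grass support actor from the procedural road generator that dresses three static mesh components with tree meshes picked from an array.
; The Construction Script does all the work, reseeding the random stream only when the RandomizeTree toggle is set, then clearing it like a button.
; Each component adds a fixed offset to the initial seed, so picks are repeatable yet can differ per slot.
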(event EventBeginPlay)

(event Collision|EventActorBeginOverlap
  (params (OtherActor :type Actor%20Object%20Reference)))

(event EventTick
  (params (DeltaSeconds :type Float%20%28single-precision%29)))

(fn ConstructionScript
  (Utilities|FlowControl|Sequence
    (:then_0
      (if (Variables|Default|GetRandomize%20Tree)
        (Class|KismetMathLibrary|SeedRandomStream (Variables|Default|GetSeed)))
      (Variables|Default|SetRandomize%20Tree false))
    (:then_1
      (bind _output_get (Variables|Default|SetNumber%20Of%20Tree%20 (Utilities|Array|Length (Variables|Default|GetTrees%20Array))))
      (if (> _output_get 0)
        (Components|StaticMesh|SetStaticMesh (Variables|Default|GetBridge_Side_Grass_Support2) (CallFunction|GetRandomTree))
        (Components|StaticMesh|SetStaticMesh (Variables|Default|GetBridge_Side_Grass_Support3) (CallFunction|GetRandomTree 45))
        (Components|StaticMesh|SetStaticMesh (Variables|Default|GetBridge_Side_Grass_Support1) (CallFunction|GetRandomTree 23))))))

(fn GetRandomTree
  (params (Seed%20Iteration :type Integer))
  (return (Utilities|Array|Get(acopy) (Variables|Default|GetTrees%20Array) (Math|Random|RandomIntegerinRangefromStream 0 (- (Variables|Default|GetNumber%20Of%20Tree%20) 1) (Math|Random|MakeRandomStream (+ Seed%20Iteration (.initialseed (Variables|Default|GetSeed))))))))