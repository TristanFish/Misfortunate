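; Light actor in the procedural road generator that pairs a RectLight with a LightBox mesh in a matching random color.
; The Construction Script builds the color from three seeded streams, one per RGB channel, and applies it to the light and a dynamic glass material on the box.
; RandomizeLightColor acts as a one-shot toggle that reseeds the streams and resets itself.
; The event graph has no active logic.
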(event EventBeginPlay)

(event Collision|EventActorBeginOverlap
  (params (OtherActor :type Actor%20Object%20Reference)))

(event EventTick
  (params (DeltaSeconds :type Float%20%28single-precision%29)))

(fn ConstructionScript
  (Utilities|FlowControl|Sequence
    (:then_0
      (if (Variables|Default|GetRandomize%20Light%20Color)
        (Class|KismetMathLibrary|SeedRandomStream (Variables|Default|GetRed%20Seed))
        (Class|KismetMathLibrary|SeedRandomStream (Variables|Default|GetGreen%20Seed))
        (Class|KismetMathLibrary|SeedRandomStream (Variables|Default|GetBlue%20Seed))
        (Variables|Default|SetRandomize%20Light%20Color false)))
    (:then_1
      (LocalVariables|SetColor (Math|Color|MakeColor (Math|Random|RandomFloatinRangefromStream 0.2 1.0 (Math|Random|MakeRandomStream (.initialseed (Variables|Default|GetRed%20Seed)))) (Math|Random|RandomFloatinRangefromStream 0.2 1.0 (Math|Random|MakeRandomStream (.initialseed (Variables|Default|GetGreen%20Seed)))) (Math|Random|RandomFloatinRangefromStream 0.2 1.0 (Math|Random|MakeRandomStream (.initialseed (Variables|Default|GetBlue%20Seed))))))
      (Rendering|Components|Light|SetLightColor (Variables|Default|GetRectLight) (LocalVariables|GetColor) true)
      (bind _returnvalue (Rendering|Material|CreateDynamicMaterialInstance (Variables|Default|GetLight_Box) 0 "/Game/ProceduralRoadGenerator/Material/Glass/Opaque_Glass_inst5.Opaque_Glass_inst5" "None" :!class /Script/Engine.PrimitiveComponent))
      (Rendering|Material|SetVectorParameterValue _returnvalue "Uniform Color" (LocalVariables|GetColor) :!class /Script/Engine.MaterialInstanceDynamic))))