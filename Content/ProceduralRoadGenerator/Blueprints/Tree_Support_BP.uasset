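; Tree support actor for the procedural road generator that varies the material on its decal.
; The construction script picks a material from DecalMaterials using the MaterialSeed random stream.
; RandomizeDecalMaterial acts as a one-shot editor toggle: when set, it reseeds the stream and clears itself, so the chosen material otherwise follows the stored seed.
; The event graph has no active logic.
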(event EventBeginPlay)

(event Collision|EventActorBeginOverlap
  (params (OtherActor :type Actor%20Object%20Reference)))

(event EventTick
  (params (DeltaSeconds :type Float%20%28single-precision%29)))

(fn ConstructionScript
  ;[1 1 1] Set Random Decal Material
  (Utilities|FlowControl|Sequence
    (:then_0
      (if (Variables|Default|GetRandomize%20Decal%20Material)
        (Class|KismetMathLibrary|SeedRandomStream (Variables|Default|GetMaterial%20Seed)))
      (Variables|Default|SetRandomize%20Decal%20Material false))
    (:then_1
      (Rendering|Components|Decal|SetDecalMaterial (Variables|Default|GetDecal) (Utilities|Array|Get(acopy) (Variables|Default|GetDecal%20Materials) (Math|Random|RandomIntegerinRangefromStream 0 (- (Utilities|Array|Length (Variables|Default|GetDecal%20Materials)) 1) (Variables|Default|GetMaterial%20Seed)))))))