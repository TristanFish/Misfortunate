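; Sky sphere actor with an optional animated day-night cycle that drives the sky material, sun light and fog.
; Construction builds a dynamic sky material, applies time-of-day settings and pushes global values to a Material Parameter Collection.
; At runtime a timeline rotates the directional light, deriving sun height to sample color curves and adjust intensity and shadows.
; Tick, throttled by a configurable interval, recaptures the skylight and recolors fog.
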(event Custom|Update%20SkyLight
  (bind _exponential_fog_actor (Variables|Default|GetExponential%20Fog%20Actor))
  (bind _sun_height (Variables|Overridesettings|GetSun%20height))
  (bind _horizon_color_curve (Variables|Default|GetHorizon%20color%20curve))
  (bind _returnvalue (Math|Curves|GetLinearColorValue _horizon_color_curve _sun_height))
  (bind _component (Variables|/Script/Engine.ExponentialHeightFog|GetComponent _exponential_fog_actor))
  (Utilities|FlowControl|Sequence
    (:then_0
      ;[1 1 1] Check if Valid
      (Utilities|FlowControl|DoOnce false
        (:Completed
          (Utilities|IsValid (Variables|Default|GetSkyLight)
            (:Is%20Valid
              (Variables|Default|SetIs%20Sky%20Light%20Valid true))
            (:Is%20Not%20Valid
              (Variables|Default|SetIs%20Sky%20Light%20Valid false)))
          (Utilities|IsValid (Variables|Default|GetExponential%20Fog%20Actor)
            (:Is%20Valid
              (Variables|Default|SetIs%20Exponential%20fog%20Valid true))
            (:Is%20Not%20Valid
              (Variables|Default|SetIs%20Exponential%20fog%20Valid false))))))
    (:then_1
      (if (Variables|Default|GetIs%20Sky%20Light%20Valid)
        (Class|SkyLightComponent|RecaptureSky (Variables|/Script/Engine.SkyLight|GetLightComponent (Variables|Default|GetSkyLight)))))
    (:then_2
      (if (Variables|Default|GetIs%20Exponential%20fog%20Valid)
        (Class|ExponentialHeightFogComponent|SetFogInscatteringColor _component _returnvalue)
        (Class|ExponentialHeightFogComponent|SetDirectionalInscatteringColor _component _returnvalue)))))

(event EventTick
  (params (DeltaSeconds :type Float%20%28single-precision%29))
  ;[1 1 1] Event Tick /// sky light recapture
  (if (and (Variables|EScenelighting|GetActivateDayNightCycle?) (not (Variables|Default|GetHide%20The%20Sky%20Sphere)))
    (Actor|Tick|SetActorTickInterval (Variables|GameSettings|GetSky%20Reflection%20Update%20Speed%20%28tick%20intervall%29))
    (CallFunction|UpdateSkyLight)))

(event EventBeginPlay
  (bind _directional_light_actor (Variables|Default|GetDirectional%20light%20actor))
  (bind _returnvalue (Transformation|GetActorRotation _directional_light_actor))
  (bind (_roll _pitch _yaw) (Math|Rotator|BreakRotator _returnvalue))
  (CallFunction|InitializeGlobalMaterialSettings)
  (if (and (Variables|EScenelighting|GetActivateDayNightCycle?) (not (Variables|Default|GetHide%20The%20Sky%20Sphere)))
    (Utilities|IsValid (Variables|Default|GetDirectional%20light%20actor)
      (:Is%20Valid
        ;[1 1 1] Day Night Cycle
        (Utilities|FlowControl|Sequence
          (:then_0
            (Utilities|FlowControl|DoOnce false
              (:Completed
                (Variables|Default|SetCurrentLightIntensity (Variables|/Script/Engine.LightComponentBase|GetIntensity (Variables|/Script/Engine.Light|GetLightComponent (Variables|Default|GetDirectional%20light%20actor)))))))
          (:then_1
            (if (Variables|EScenelighting|GetActivateDayNightCycle?)
              (bind _sun_position (Timeline|Timeline_0 Play)
                (:Update
                  (bind _output_get (Variables|EScenelighting|SetSun%20position%20Y%20output (+ (* (Variables|EScenelighting|GetSpeed%20Update%20Factor) _sun_position) (Variables|EScenelighting|GetSun%20position%20%28Y%29%20%28Time%20Of%20Day%29))))
                  (Transformation|SetActorRotation (Variables|Default|GetDirectional%20light%20actor) (Math|Rotator|MakeRotator (Variables|EScenelighting|GetSun%20Roll%20%28X%29) _output_get (Variables|EScenelighting|GetSun%20Yaw%20%28Z%29)))
                  (CallFunction|UpdateSunDirection)
                  (CallFunction|SunIntensityAtenuation (Variables|EScenelighting|GetMax%20Sun%20Light%20%20Intensity))
                  (if (Variables|EScenelighting|GetUse%20Horizon%20Color%20as%20Sun%20Light%20Color)
                    (Rendering|Components|Light|SetLightColor (Variables|/Script/Engine.Light|GetLightComponent (Variables|Default|GetDirectional%20light%20actor)) (Math|Curves|GetLinearColorValue (Variables|Default|GetHorizon%20color%20curve) (Variables|Overridesettings|GetSun%20height)) true)))
                (:Finished
                  (Transformation|SetActorRotation _directional_light_actor (Math|Rotator|MakeRotator _roll _pitch (+ _yaw (Variables|EScenelighting|GetSun%20Yaw%20%28Z%29%20Cycle%20rot))))
                  (Variables|EScenelighting|SetSun%20position%20Y%20output 0.0))))))))))

(fn ConstructionScript
  (bind _directional_light_actor (Variables|Default|GetDirectional%20light%20actor))
  (bind _exponential_fog_actor (Variables|Default|GetExponential%20Fog%20Actor))
  (bind _skylight (Variables|Default|GetSkyLight))
  (bind _directional_light_actor_2 (Variables|Default|GetDirectional%20light%20actor))
  (bind _lightcomponent (Variables|/Script/Engine.Light|GetLightComponent _directional_light_actor_2))
  (bind _component (Variables|/Script/Engine.ExponentialHeightFog|GetComponent _exponential_fog_actor))
  (CallFunction|InitializeGlobalMaterialSettings)
  (if (Variables|Default|GetHide%20The%20Sky%20Sphere)
    (Rendering|SetVisibility (Variables|BP_Skydome|GetBase) false false)
    (else
      (Rendering|SetVisibility (Variables|BP_Skydome|GetBase) true false)
      (Utilities|FlowControl|Sequence
        (:then_0
          (Utilities|IsValid _skylight
            (:Is%20Valid
              (if (Variables|EScenelighting|GetAuto%20Update%20Sky%20Light)
                (Class|SkyLightComponent|RecaptureSky (Variables|/Script/Engine.SkyLight|GetLightComponent _skylight))))
            (:Is%20Not%20Valid
              _))
          (bind _returnvalue (Rendering|Material|CreateDynamicMaterialInstance (Variables|BP_Skydome|GetSky%20Sphere%20mesh) 0 "/Engine/EngineSky/M_Sky_Panning_Clouds2.M_Sky_Panning_Clouds2" "None" :!class /Script/Engine.PrimitiveComponent))
          (Variables|Default|SetSky%20material _returnvalue)
          (Utilities|FlowControl|Sequence
            (:then_0
              _)
            (:then_1
              (Utilities|IsValid _directional_light_actor
                (:Is%20Valid
                  (Transformation|SetActorRotation _directional_light_actor (Math|Rotator|MakeRotator (Variables|EScenelighting|GetSun%20Roll%20%28X%29) (Variables|EScenelighting|GetSun%20position%20%28Y%29%20%28Time%20Of%20Day%29) (Variables|EScenelighting|GetSun%20Yaw%20%28Z%29)))))))
          (if (Variables|EScenelighting|GetRefresh%20material) ; Updating bool in details panel causes construction script to run again
            _
            (else
              _))
          (Variables|EScenelighting|SetRefresh%20material false)
          (Rendering|Material|SetScalarParameterValue (Variables|Default|GetSky%20material) "Sun Radius" (Variables|EScenelighting|GetSun%20Radius) :!class /Script/Engine.MaterialInstanceDynamic)
          (Utilities|IsValid (Variables|Default|GetDirectional%20light%20actor) ; Has a directional light been assigned?
            (:Is%20Valid
              (Rendering|Components|Light|SetLightColor (Variables|/Script/Engine.Light|GetLightComponent (Variables|Default|GetDirectional%20light%20actor)) (Variables|EScenelighting|GetSun%20Color) true)
              (Rendering|Material|SetVectorParameterValue (Variables|Default|GetSky%20material) "Light direction" (Math|Conversions|ToLinearColor(Vector) (Math|Rotator|GetRotationXVector (Transformation|GetActorRotation (Variables|Default|GetDirectional%20light%20actor)))) :!class /Script/Engine.MaterialInstanceDynamic)
              (Rendering|Material|SetVectorParameterValue (Variables|Default|GetSky%20material) "Sun color" (Math|Conversions|ToLinearColor(Color) (Variables|/Script/Engine.LightComponentBase|GetLightColor (Variables|/Script/Engine.Light|GetLightComponent (Variables|Default|GetDirectional%20light%20actor)))) :!class /Script/Engine.MaterialInstanceDynamic)
              (Variables|Overridesettings|SetSun%20height (Math|Float|MapRangeUnclamped (.Pitch (Math|Rotator|BreakRotator (Transformation|GetActorRotation (Variables|Default|GetDirectional%20light%20actor)))) 0.0 -9e+01 0.0 1.0)))
            (:Is%20Not%20Valid
              (Rendering|Material|SetVectorParameterValue (Variables|Default|GetSky%20material) "Light direction" (Math|Conversions|ToLinearColor(Vector) (Math|Rotator|GetRotationXVector (Math|Rotator|MakeRotator 0.0 (Math|Float|MapRangeUnclamped (Variables|Overridesettings|GetSun%20height) -1.0 1.0 9e+01 -9e+01) (.Yaw (Math|Rotator|BreakRotator (Transformation|GetActorRotation)))))) :!class /Script/Engine.MaterialInstanceDynamic)
              (Rendering|Material|SetVectorParameterValue (Variables|Default|GetSky%20material) "Sun color" (Math|Color|Lerp(LinearColor) "(R=1.000000,G=0.221000,B=0.040000,A=1.000000)" "(R=0.954000,G=0.901000,B=0.744120,A=1.000000)" (Math|Float|Clamp(Float) (+ (Variables|Overridesettings|GetSun%20height) 0.2))) :!class /Script/Engine.MaterialInstanceDynamic)))
          (if (Variables|EScenelighting|GetColors%20determined%20by%20sun%20position)
            (Rendering|Material|SetVectorParameterValue (Variables|Default|GetSky%20material) "Horizon color" (Math|Curves|GetLinearColorValue (Variables|Default|GetHorizon%20color%20curve) (Variables|Overridesettings|GetSun%20height)) :!class /Script/Engine.MaterialInstanceDynamic)
            (Rendering|Material|SetVectorParameterValue (Variables|Default|GetSky%20material) "Zenith color" (Math|Curves|GetLinearColorValue (Variables|Default|GetZenith%20color%20curve) (Variables|Overridesettings|GetSun%20height)) :!class /Script/Engine.MaterialInstanceDynamic)
            (Rendering|Material|SetVectorParameterValue (Variables|Default|GetSky%20material) "Cloud color" (Math|Curves|GetLinearColorValue (Variables|Default|GetCloud%20color%20curve) (Variables|Overridesettings|GetSun%20height)) :!class /Script/Engine.MaterialInstanceDynamic)
            (Rendering|Material|SetScalarParameterValue (Variables|Default|GetSky%20material) "Horizon falloff" (Math|Float|Lerp 3.0 7.0 (Math|Float|Absolute(Float) (Variables|Overridesettings|GetSun%20height))) :!class /Script/Engine.MaterialInstanceDynamic)
            (else
              (Rendering|Material|SetVectorParameterValue (Variables|Default|GetSky%20material) "Horizon color" (Variables|Overridesettings|GetHorizon%20color) :!class /Script/Engine.MaterialInstanceDynamic)
              (Rendering|Material|SetVectorParameterValue (Variables|Default|GetSky%20material) "Zenith color" (Variables|Overridesettings|GetZenith%20Color) :!class /Script/Engine.MaterialInstanceDynamic)
              (Rendering|Material|SetVectorParameterValue (Variables|Default|GetSky%20material) "Overall color" (Variables|Overridesettings|GetOverall%20Color) :!class /Script/Engine.MaterialInstanceDynamic)
              (Rendering|Material|SetVectorParameterValue (Variables|Default|GetSky%20material) "Cloud color" (Variables|Overridesettings|GetCloud%20color) :!class /Script/Engine.MaterialInstanceDynamic)
              (Rendering|Material|SetScalarParameterValue (Variables|Default|GetSky%20material) "Horizon falloff" (Variables|Overridesettings|GetHorizon%20Falloff) :!class /Script/Engine.MaterialInstanceDynamic)))
          (Rendering|Material|SetScalarParameterValue (Variables|Default|GetSky%20material) "Cloud speed" (Variables|EScenelighting|GetCloud%20speed) :!class /Script/Engine.MaterialInstanceDynamic)
          (Rendering|Material|SetScalarParameterValue (Variables|Default|GetSky%20material) "Sun brightness" (Variables|EScenelighting|GetSun%20brightness) :!class /Script/Engine.MaterialInstanceDynamic)
          (Rendering|Material|SetScalarParameterValue (Variables|Default|GetSky%20material) "Sun height" (Math|Float|SelectFloat (Math|Float|Absolute(Float) (Variables|Overridesettings|GetSun%20height)) 0.0 (< (Variables|Overridesettings|GetSun%20height) 0.0)) :!class /Script/Engine.MaterialInstanceDynamic)
          (Rendering|Material|SetScalarParameterValue (Variables|Default|GetSky%20material) "Cloud opacity" (Variables|EScenelighting|GetCloud%20opacity) :!class /Script/Engine.MaterialInstanceDynamic)
          (Rendering|Material|SetScalarParameterValue (Variables|Default|GetSky%20material) "Stars brightness" (Variables|EScenelighting|GetStars%20brightness) :!class /Script/Engine.MaterialInstanceDynamic))
        (:then_1
          ;[1 1 1] Set Expo Fog
          (Utilities|IsValid (Variables|Default|GetExponential%20Fog%20Actor)
            (:Is%20Valid
              (Class|ExponentialHeightFogComponent|SetFogInscatteringColor _component (Math|Curves|GetLinearColorValue (Variables|Default|GetHorizon%20color%20curve) (Variables|Overridesettings|GetSun%20height)))
              (Class|ExponentialHeightFogComponent|SetDirectionalInscatteringColor _component (Math|Curves|GetLinearColorValue (Variables|Default|GetHorizon%20color%20curve) (Variables|Overridesettings|GetSun%20height))))))
        (:then_2
          ;[1 1 1] Set Sun Color and bloom
          (Utilities|IsValid (Variables|Default|GetDirectional%20light%20actor)
            (:Is%20Valid
              (if (Variables|EScenelighting|GetUse%20Horizon%20Color%20as%20Sun%20Light%20Color)
                (Rendering|Components|Light|SetLightColor _lightcomponent (Math|Curves|GetLinearColorValue (Variables|Default|GetHorizon%20color%20curve) (Variables|Overridesettings|GetSun%20height)) true)
                (Class|LightComponent|SetBloomTint _lightcomponent (Math|Conversions|ToColor(LinearColor) (Math|Curves|GetLinearColorValue (Variables|Default|GetHorizon%20color%20curve) (Variables|Overridesettings|GetSun%20height)))))
              (CallFunction|SunIntensityAtenuation (Variables|EScenelighting|GetMax%20Sun%20Light%20%20Intensity)))))))))

(fn UpdateSunDirection
  (bind _sky_material (Variables|Default|GetSky%20material))
  (bind _sky_material_2 (Variables|Default|GetSky%20material))
  (Utilities|FlowControl|Sequence
    (:then_0
      (Utilities|FlowControl|DoOnce false
        (:Completed
          (Utilities|IsValid (Variables|Default|GetDirectional%20light%20actor)
            (:Is%20Valid
              (Variables|Default|SetIs%20Directionnal%20Light%20Valid true))
            (:Is%20Not%20Valid
              (Variables|Default|SetIs%20Directionnal%20Light%20Valid false))))))
    (:then_1
      (if (Variables|Default|GetIs%20Directionnal%20Light%20Valid)
        (Rendering|Material|SetVectorParameterValue _sky_material "Light direction" (Math|Conversions|ToLinearColor(Vector) (Math|Rotator|GetRotationXVector (Transformation|GetActorRotation (Variables|Default|GetDirectional%20light%20actor)))) :!class /Script/Engine.MaterialInstanceDynamic)
        (Rendering|Material|SetVectorParameterValue _sky_material "Sun color" (Math|Conversions|ToLinearColor(Color) (Variables|/Script/Engine.LightComponentBase|GetLightColor (Variables|/Script/Engine.Light|GetLightComponent (Variables|Default|GetDirectional%20light%20actor)))) :!class /Script/Engine.MaterialInstanceDynamic)
        (Variables|Overridesettings|SetSun%20height (Math|Float|MapRangeUnclamped (.Pitch (Math|Rotator|BreakRotator (Transformation|GetActorRotation (Variables|Default|GetDirectional%20light%20actor)))) 0.0 -9e+01 0.0 1.0))
        (Rendering|Material|SetVectorParameterValue _sky_material_2 "Horizon color" (Math|Curves|GetLinearColorValue (Variables|Default|GetHorizon%20color%20curve) (Variables|Overridesettings|GetSun%20height)) :!class /Script/Engine.MaterialInstanceDynamic)
        (Rendering|Material|SetVectorParameterValue _sky_material_2 "Zenith color" (Math|Curves|GetLinearColorValue (Variables|Default|GetZenith%20color%20curve) (Variables|Overridesettings|GetSun%20height)) :!class /Script/Engine.MaterialInstanceDynamic)
        (Rendering|Material|SetVectorParameterValue _sky_material_2 "Cloud color" (Math|Curves|GetLinearColorValue (Variables|Default|GetCloud%20color%20curve) (Variables|Overridesettings|GetSun%20height)) :!class /Script/Engine.MaterialInstanceDynamic)
        (Rendering|Material|SetScalarParameterValue _sky_material_2 "Horizon falloff" (Math|Float|Lerp 3.0 8.0 (Math|Float|Absolute(Float) (Variables|Overridesettings|GetSun%20height))) :!class /Script/Engine.MaterialInstanceDynamic)
        (Rendering|Material|SetScalarParameterValue _sky_material_2 "Sun height" (Math|Float|SelectFloat (Math|Float|Absolute(Float) (Variables|Overridesettings|GetSun%20height)) 0.0 (< (Variables|Overridesettings|GetSun%20height) 0.0)) :!class /Script/Engine.MaterialInstanceDynamic)))))

(fn SunIntensityAtenuation
  (params (Max%20Sun%20Light%20Intensity :type Float%20%28single-precision%29))
  (bind _sun_height (Variables|Overridesettings|GetSun%20height))
  (bind _sun_height_2 (Variables|Overridesettings|GetSun%20height))
  (bind _directional_light_actor (Variables|Default|GetDirectional%20light%20actor))
  (bind _min_sun_light__intensity (Variables|EScenelighting|GetMin%20Sun%20Light%20%20Intensity))
  (bind _returnvalue (Math|Float|Clamp(Float) _min_sun_light__intensity 0.0 Max%20Sun%20Light%20Intensity))
  (bind _lightcomponent (Variables|/Script/Engine.Light|GetLightComponent _directional_light_actor))
  (Rendering|Components|Light|SetIntensity (Variables|/Script/Engine.Light|GetLightComponent (Variables|Default|GetDirectional%20light%20actor)) (select (>= _sun_height 0.0) (Math|Float|Lerp _returnvalue Max%20Sun%20Light%20Intensity (Math|Float|Absolute(Float) _sun_height)) _returnvalue))
  (if (not (and (<= -0.457143 _sun_height_2) (>= _sun_height_2 -0.011111)))
    (Rendering|Components|Light|SetCastShadows _lightcomponent false)
    (else
      (Rendering|Components|Light|SetCastShadows _lightcomponent true))))

(fn InitializeGlobalMaterialSettings
  (Rendering|Material|SetScalarParameterValue "/Game/ProceduralRoadGenerator/Material_Functions/Global_Params.Global_Params" "G_Roughness Intensity" (Variables|GlobalMaterialSettings|GetGlobal%20Roughness%20Multiplier) :!class /Script/Engine.KismetMaterialLibrary)
  (Rendering|Material|SetScalarParameterValue "/Game/ProceduralRoadGenerator/Material_Functions/Global_Params.Global_Params" "G_Light Intensity" (Variables|GlobalMaterialSettings|GetGlobal%20Light%20Intensity%20Multiplier) :!class /Script/Engine.KismetMaterialLibrary)
  (Rendering|Material|SetScalarParameterValue "/Game/ProceduralRoadGenerator/Material_Functions/Global_Params.Global_Params" "G_Light_Switch" (Variables|GlobalMaterialSettings|GetGlobal%20Light%20switching) :!class /Script/Engine.KismetMaterialLibrary))