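; Player character Blueprint for Misfortuante, handling the headlamp, heartbeat audio and lore tablet detection.
; BeginPlay silences the heartbeat, then spawns a headlamp and attaches it to the camera.
; UpdateHeartBeatAudio combines low Stamina and high Misfortune into the HeartBeatSpeed sound parameter, with a debug print.
; Tick runs a short debug-drawn camera trace, telling MPlayerController to show or hide the tablet interaction prompt.
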(event EventBeginPlay
  (Audio|Components|Audio|Stop (Variables|Default|GetheartbeatAudio))
  (bind _returnvalue (Game|SpawnActorfromClass "/Game/Misfortuante/Blueprints/Actors/HeadLampComp.HeadLampComp_C" (Math|Transform|MakeTransform "0, 0, 0" "0, 0, 0" "1.000000,1.000000,1.000000") "Undefined" "MultiplyWithRoot" 0 0))
  (bind _output_get (Variables|Default|SetHeadLamp _returnvalue))
  (Variables|/Script/Misfortunate.HeadLamp|SetOnOffSound _output_get "/Game/Misfortuante/Audio/Flashlight_OnOff_Cue.Flashlight_OnOff_Cue")
  (Transformation|AttachComponentToComponent _output_get (Variables|Default|GetplayerCamera) "None" "SnapToTarget" "SnapToTarget" "SnapToTarget" true)
  (Transformation|SetActorRelativeLocation (Variables|Default|GetHeadLamp) "3.000000, 0,18.000000"))

(event EventUpdateHeartBeatAudio
  (bind _stamina (Variables|Default|GetStamina))
  (bind _misfortune (Variables|Default|GetMisfortune))
  (bind _returnvalue (Math|Float|MapRangeClamped _misfortune 0.0 1e+02 0.0 8.0))
  (bind _returnvalue_2 (Math|Float|MapRangeClamped _stamina 0.0 1e+02 8.0 0.0))
  (bind _returnvalue_3 (+ _returnvalue_2 _returnvalue))
  (bind _returnvalue_4 (Math|Float|MapRangeClamped _returnvalue_3 0.0 16.0 0.0 8.0))
  (Development|PrintString (Utilities|String|ToString(Float) _returnvalue_4))
  (Audio|Parameter|SetFloatParameter (Variables|Default|GetheartbeatAudio) "HeartBeatSpeed" _returnvalue_4 :!class /Script/AudioExtensions.AudioParameterControllerInterface))

(event EventTick
  (params (DeltaSeconds :type Float%20%28single-precision%29))
  (bind _returnvalue (Pawn|GetController))
  (bind _playercamera (Variables|Default|GetplayerCamera))
  (bind _returnvalue_2 (Transformation|GetWorldLocation _playercamera))
  (bind (_outhit _returnvalue_3) (Collision|LineTraceByChannel _returnvalue_2 (+ (* (Math|Vector|GetForwardVector (Variables|Default|GetplayerCamera)) 2e+02) _returnvalue_2) "TraceTypeQuery1" false 0 "ForOneFrame"))
  (if _returnvalue_3
    (bind _aslore_tablet_generic (Utilities|Casting|CastToLoreTablet_Generic (.HitActor (Collision|BreakHitResult _outhit)))
      (:then
        (bind _asmplayer_controller (Utilities|Casting|CastToMPlayerController _returnvalue))
        (Class|MPlayerController|DisplayTabletInteraction _asmplayer_controller _aslore_tablet_generic))
      (:CastFailed
        (bind _asmplayer_controller_2 (Utilities|Casting|CastToMPlayerController _returnvalue :!label _label))
        (Class|MPlayerController|HideInteraction _asmplayer_controller_2)))
    (else
      (goto _label))))

(fn ConstructionScript)