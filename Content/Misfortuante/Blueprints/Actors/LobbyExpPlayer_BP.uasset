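; Player Blueprint, named for the lobby, that equips a camera-mounted headlamp and drives heartbeat audio.
; BeginPlay silences the heartbeat, spawns the HeadLamp actor, assigns its flashlight toggle sound and snaps it to PlayerCamera with a small offset.
; UpdateHeartBeatAudio sums range-mapped Stamina and Misfortune into the HeartBeatSpeed sound parameter, so lower stamina and higher misfortune raise the rate.
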(event EventBeginPlay
  (Audio|Components|Audio|Stop (Variables|Default|GetheartbeatAudio))
  (bind _returnvalue (Game|SpawnActorfromClass "/Game/Misfortuante/Blueprints/Actors/HeadLampComp.HeadLampComp_C" (Math|Transform|MakeTransform "0, 0, 0" "0, 0, 0" "1.000000,1.000000,1.000000") "Undefined" "MultiplyWithRoot" 0 0))
  (bind _output_get (Variables|Default|SetHeadLamp _returnvalue))
  (Variables|/Script/Misfortunate.HeadLamp|SetOnOffSound _output_get "/Game/Misfortuante/Audio/Flashlight_OnOff_Cue.Flashlight_OnOff_Cue")
  (Transformation|AttachComponentToComponent _returnvalue (Variables|Default|GetplayerCamera) "None" "SnapToTarget" "SnapToTarget" "SnapToTarget" true)
  (Transformation|SetActorRelativeLocation _returnvalue "3.000000, 0,18.000000"))

(event Collision|EventActorBeginOverlap
  (params (OtherActor :type Actor%20Object%20Reference)))

(event EventTick
  (params (DeltaSeconds :type Float%20%28single-precision%29)))

(event EventUpdateHeartBeatAudio
  (Audio|Parameter|SetFloatParameter (Variables|Default|GetheartbeatAudio) "HeartBeatSpeed" (Math|Float|MapRangeClamped (+ (Math|Float|MapRangeClamped (Variables|Default|GetStamina) 0.0 1e+02 8.0 0.0) (Math|Float|MapRangeClamped (Variables|Default|GetMisfortune) 0.0 1e+02 0.0 8.0)) 0.0 16.0 0.1 8.0) :!class /Script/AudioExtensions.AudioParameterControllerInterface))

(fn ConstructionScript)