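; Game instance for a multiplayer game that manages Steam player info and hosting, finding and joining sessions through Advanced Sessions.
; On Init it fetches the local player's name and Steam avatar, then registers the name as the ServerName session setting.
; Hosting opens FirstPersonExampleMap as a listen server, while searches cache results in ActiveSessions and refresh the games list widget.
; Joins, failed searches, and travel or network errors only print debug messages.
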(event EventHostSession
  (|AdvancedSession (Variables|Default|GetServerSettings) (Game|GetPlayerController 0) 100 4 false true false true true false false false true
    (:OnSuccess
      (Game|OpenLevel(byName) "FirstPersonExampleMap" true "listen"))))

(event EventJoinActiveSession
  (params (Session :type Blueprint%20Session%20Result%20Structure%20%28by%20ref%29))
  (|JoinSession (Game|GetPlayerController 0) Session
    (:OnSuccess
      (Development|PrintString "Joined Session"))
    (:OnFailure
      (Development|PrintString "Failed To Join Session"))))

(event EventUpdateActiveSessions
  (params (W_ActiveGames :type W%20Active%20Games%20Object%20Reference))
  (Utilities|Array|Clear (Variables|Default|GetActiveSessions))
  (bind _results (|FindSessionsAdvanced (Game|GetPlayerController 0) 50 false "AllServers" 0 false false false)
    (:OnSuccess
      (Variables|Default|SetActiveSessions _results)
      (Class|WActiveGames|UpdateGamesScrollBox W_ActiveGames))
    (:OnFailure
      (Development|PrintString "Failed"))))

(event EventInit
  (bind _returnvalue (Game|GetPlayerController 0))
  (bind _playername (Class|AdvancedSessionsLibrary|GetPlayerName _returnvalue))
  (bind _returnvalue_2 (Class|AdvancedSteamFriendsLibrary|GetSteamFriendAvatar (Class|AdvancedSessionsLibrary|GetUniqueNetID _returnvalue) "SteamAvatar_Medium")
    (:OnSuccess
      (Variables|Default|SetPlayerInfo (Utilities|Struct|MakePlayerInfo _playername _returnvalue_2))
      (Utilities|Array|AddUnique (Variables|Default|GetServerSettings) (Class|AdvancedSessionsLibrary|MakeLiteralSessionPropertyString "ServerName" _playername))
      (Development|PrintString "Game Instance Init Called" true true "(R=0.000000,G=0.660000,B=1.000000,A=1.000000)" 5.0))))

(event EventHandleTravelError
  (params (FailureType :type ETravelFailure%20Enum :default "NoLevel"))
  (Development|PrintString (Utilities|String|Append "Travel Error: " (Utilities|String|EnumtoString FailureType)) true true "(R=0.000000,G=0.660000,B=1.000000,A=1.000000)" 1e+01))

(event EventHandleNetworkError
  (params (FailureType :type ENetworkFailure%20Enum :default "NetDriverAlreadyExists") (bIsServer :type Boolean))
  (Development|PrintString (Utilities|String|Append "Network Error: " (Utilities|String|EnumtoString FailureType)) true true "(R=0.000000,G=0.660000,B=1.000000,A=1.000000)" 1e+01))

(fn GetActiveSessions
  (return (Variables|Default|GetActiveSessions)))