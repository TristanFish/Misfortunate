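; Game instance for Misfortunate that handles multiplayer session hosting, searching and joining through Advanced Sessions, and logs travel and network errors.
; Init builds the local player's info from their name and Steam avatar and adds a ServerName setting.
; Hosting creates a session and opens the first-person map as a listen server.
; Searches store results, remove entries lacking ServerName by index, then refresh the active-games widget's list.
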(event EventHostSession
  (Utilities|Array|Add (Variables|Default|GetServerSettings) (Class|AdvancedSessionsLibrary|MakeLiteralSessionPropertyString "ServerName" "Testing"))
  (|AdvancedSession (Variables|Default|GetServerSettings) (Game|GetPlayerController 0) 100 4 false true false true true true false false false true false true
    (:OnSuccess
      (Game|OpenLevel(byName) "FirstPersonExampleMap" true "listen"))))

(event EventJoinActiveSession
  (params (Session :type Blueprint%20Session%20Result%20Structure%20%28by%20ref%29))
  (|JoinSession (Game|GetPlayerController 0) Session
    (:OnSuccess
      (Development|PrintString "Successfully Joined Session"))
    (:OnFailure
      (Development|PrintString "Failed To Join Session"))))

(event EventUpdateActiveSessions
  (params (W_ActiveGames :type W%20Active%20Games%20Object%20Reference))
  (Utilities|Array|Clear (Variables|Default|GetActiveSessions))
  (bind _results (|FindSessionsAdvanced (Game|GetPlayerController 0) 1000 false "AllServers" 0 false false false true)
    (:OnSuccess
      (bind _output_get (Variables|Default|SetTempActiveSessions _results))
      (Variables|Default|SetActiveSessions _results)
      (for (_array_element _array_index) _output_get
        (bind _extrasettings (Class|AdvancedSessionsLibrary|GetExtraSettings _array_element))
        (Class|AdvancedSessionsLibrary|GetSessionPropertyString _extrasettings "ServerName"
          (:NotFound
            (Utilities|Array|RemoveIndex (Variables|Default|GetActiveSessions) _array_index))))
      (Class|WActiveGames|UpdateGamesScrollBox W_ActiveGames))
    (:OnFailure
      (Development|PrintString "Failed"))))

(event EventInit
  (bind _returnvalue (Game|GetPlayerController 0))
  (bind _playername (Class|AdvancedSessionsLibrary|GetPlayerName _returnvalue))
  (bind _returnvalue_2 (Class|AdvancedSteamFriendsLibrary|GetSteamFriendAvatar (Class|AdvancedSessionsLibrary|GetUniqueNetID _returnvalue) "SteamAvatar_Medium")
    (:OnSuccess
      (Variables|Default|SetPlayerInfo (Utilities|Struct|MakePlayerInfo _playername _returnvalue_2 "" false))
      (Utilities|Array|AddUnique (Variables|Default|GetServerSettings) (Class|AdvancedSessionsLibrary|MakeLiteralSessionPropertyString "ServerName" _playername))
      (Development|PrintString "Game Instance Init Called" true true "(R=0.000000,G=0.660000,B=1.000000,A=1.000000)" 5.0))))

(event EventHandleTravelError
  (params (FailureType :type ETravelFailure%20Enum :default "NoLevel"))
  (Development|PrintString (Utilities|String|Append "Travel Error: " (Utilities|String|EnumtoString FailureType)) true true "(R=0.000000,G=0.660000,B=1.000000,A=1.000000)" 1e+01))

(event EventHandleNetworkError
  (params (FailureType :type ENetworkFailure%20Enum :default "NetDriverAlreadyExists") (bIsServer :type Boolean))
  (Development|PrintString (Utilities|String|Append "Network Error: " (Utilities|String|EnumtoString FailureType)) true true "(R=0.000000,G=0.660000,B=1.000000,A=1.000000)" 1e+01))

(fn GetActiveSessions
  (return (Variables|Default|GetActiveSessions)))