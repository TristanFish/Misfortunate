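; Game mode for Misfortunate that starts play in the Exploration game state and manages connected players' identity info.
; EveryoneUpdate rebuilds a list of names and net IDs from the GameState's PlayerArray, then pushes it to every connected M_PlayerController through ClientAddPlayersToList.
; InitPlayerInfo fills a given player's PlayerInfo with the name and unique net ID from its PlayerState.
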(event EventBeginPlay
  (Class|MisfortunateGameMode|SetGameState "Exploration"))

(event EventTick
  (params (DeltaSeconds :type Float%20%28single-precision%29)))

(event EventEveryoneUpdate
  (Utilities|Array|Clear (Variables|Default|GetConnectedPlayerInfos))
  (for _array_element (Variables|/Script/Engine.GameStateBase|GetPlayerArray (Game|GetGameState))
    (Utilities|Array|Add (Variables|Default|GetConnectedPlayerInfos) (Utilities|Struct|MakePlayerInfo (PlayerState|GetPlayerName _array_element) (Class|AdvancedSessionsLibrary|UniqueNetIdtoString (Class|AdvancedSessionsLibrary|GetUniqueNetIDfromPlayerState _array_element)))))
  (for _array_element_2 (Variables|Default|GetConnectedPlayers)
    (bind _asm_player_controller (Utilities|Casting|CastToM_PlayerController _array_element_2))
    (Class|MPlayerController|ClientAddPlayerstoList _asm_player_controller (Variables|Default|GetConnectedPlayerInfos))))

(event EventInitPlayerInfo
  (params (player :type M%20Player%20Controller%20Object%20Reference))
  (bind _playerstate (Variables|/Script/Engine.Controller|GetPlayerState player))
  (Variables|/Script/Misfortunate.MPlayerController|SetPlayerInfo player (Utilities|Struct|MakePlayerInfo (PlayerState|GetPlayerName _playerstate) (Class|AdvancedSessionsLibrary|UniqueNetIdtoString (Class|AdvancedSessionsLibrary|GetUniqueNetIDfromPlayerState _playerstate)))))

(fn ConstructionScript)